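; Meshless teleporter actor that moves whatever overlaps its sphere trigger to a destination actor, with an option to exclude the player.
; Overlap stores the actor and enables input, then either teleports immediately or, with InternalActivation set, waits for the placeholder F key.
; Teleporting plays sound and particles, waits a delay, then applies a yaw-based rotation.
; Automatic teleports skip actors already well inside the radius to prevent loops.
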(event OnComponentBeginOverlap(TeleportHit)
  (params (OverlappedComponent :type Primitive%20Component%20Object%20Reference) (OtherActor :type Actor%20Object%20Reference) (OtherComp :type Primitive%20Component%20Object%20Reference) (OtherBodyIndex :type Integer) (bFromSweep :type Boolean) (SweepResult :type Hit%20Result%20Structure%20%28by%20ref%29))
  (bind _teleportationplatformradius (Variables|Teleporter|GetTeleportationPlatformRadius))
  (bind _teleport_destination (Variables|Teleporter|GetTeleport%20destination))
  (bind _returnvalue (Transformation|GetActorLocation _teleport_destination))
  ;[0.9995 1 0.6033] BlockPlayer
  (if (Variables|Teleporter|GetBlockPlayer)
    (if (not (== OtherActor (Game|Player|GetPlayerPawn 0)))
      (Variables|Default|SetHitActor OtherActor :!label _label) ; Set Actor that Teleport Hits
      ;[0.7042 1 0.5929] Enable/Disable Keyboard Inputs
      (Input|EnableInput (Game|GetPlayerController 0))
      ;[0.7042 1 0.5929] Teleport by using a Activation Event
      (if (not (Variables|Teleporter|GetInternalActivation))
        (if (not (Math|Vector|Equal(Vector) (Transformation|GetActorLocation (Variables|Default|GetHitActor)) (Transformation|GetWorldLocation (Variables|Default|GetTeleportHit)) (- _teleportationplatformradius (/ _teleportationplatformradius 5e+01))))
          (if (Variables|Teleporter|GetEntryParticles)
            ;[0.228 1 0.9602] Particles for Activation
            (Effects|SpawnEmitteratLocation "/Game/Teleports/Particles/TeleportResidue.TeleportResidue" (Transformation|GetActorLocation (Variables|Default|GetHitActor)))
            (Audio|PlaySound2D "/Game/Teleports/Sound/Teleport.Teleport")
            (else
              (Audio|PlaySound2D "/Game/Teleports/Sound/Teleport.Teleport")))
          ;[0.57 0.7751 1] Teleport Actor
          (Utilities|FlowControl|Delay (Variables|Teleporter|GetTeleportationDelay))
          (Transformation|Teleport (Variables|Default|GetHitActor) _returnvalue (Utilities|TeleportObjectZRotation (Variables|Default|GetHitActor)))
          (CallFunction|ResetInput)
          ;[0.228 1 0.9602] Particles for arrival
          (Effects|SpawnEmitteratLocation "/Game/Teleports/Particles/TeleportArrival.TeleportArrival" _returnvalue))))
    (else
      (goto _label))))

(event OnComponentEndOverlap(TeleportHit)
  (params (OverlappedComponent :type Primitive%20Component%20Object%20Reference) (OtherActor :type Actor%20Object%20Reference) (OtherComp :type Primitive%20Component%20Object%20Reference) (OtherBodyIndex :type Integer))
  ;[0.9995 1 0.6033] BlockPlayer
  (if (Variables|Teleporter|GetBlockPlayer)
    (if (not (== OtherActor (Game|Player|GetPlayerPawn 0)))
      (CallFunction|ResetInput :!label _label) ; Resets the Input Event if nothing is touching the trigger box
    )
    (else
      (goto _label))))

(event Custom|Activate%20Teleport
  (bind _teleport_destination (Variables|Teleporter|GetTeleport%20destination))
  (bind _returnvalue (Transformation|GetActorLocation _teleport_destination))
  ;[0.7042 1 0.5929] Teleport by using a Activation Event
  (if (Variables|Teleporter|GetInternalActivation)
    ;[0.228 1 0.9602] Particles for Activation
    (Effects|SpawnEmitteratLocation "/Game/Teleports/Particles/TeleportResidue.TeleportResidue" (Transformation|GetActorLocation (Variables|Default|GetHitActor)))
    (Audio|PlaySound2D "/Game/Teleports/Sound/Teleport.Teleport")
    ;[0.57 0.7751 1] Teleport Actor
    (Utilities|FlowControl|Delay (Variables|Teleporter|GetTeleportationDelay))
    (Transformation|Teleport (Variables|Default|GetHitActor) _returnvalue (Utilities|TeleportObjectZRotation (Variables|Default|GetHitActor)))
    (CallFunction|ResetInput)
    ;[0.228 1 0.9602] Particles for arrival
    (Effects|SpawnEmitteratLocation "/Game/Teleports/Particles/TeleportArrival.TeleportArrival" _returnvalue)))

(event Custom|ResetInput
  ;[0.7042 1 0.5929] Enable/Disable Keyboard Inputs
  (Input|DisableInput (Game|GetPlayerController 0)))

(event Input|KeyboardEvents|F
  (params (Key :type Key%20Structure))
  ;[0.7042 1 0.5929] Activates the Teleport by Keyboard Key. Please replace with your own input Event
  (:Pressed
    (if (Variables|Teleporter|GetExternalActivation)
      ;;[0.5324 1 0.1244] Activate By external Input Event 9Teleportation Button
      (if (Variables|Default|GetMayTeleport)
        (if (!= (Variables|Default|GetHitActor) 0)
          (Audio|PlaySound2D "/Game/Teleports/Sound/ButtonClick.ButtonClick")
          (CallFunction|ActivateTeleport :!label _label)))
      (else
        (goto _label)))))

(fn ConstructionScript
  ;[1 1 1] Set Radius of Teleportation Hit Radius
  (Components|Sphere|SetSphereRadius (Variables|Default|GetTeleportHit) (Variables|Teleporter|GetTeleportationPlatformRadius) false))