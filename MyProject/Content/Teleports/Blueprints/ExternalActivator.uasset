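; ExternalActivator is a sphere trigger Blueprint that arms teleporters while something overlaps it.
; Entering its ActivateHit sphere sets MayTeleport on every Teleporter actor in the level and shows an input hint text; leaving clears both.
; Two cross-reset DoOnce nodes keep each switch to one run per enter or exit, without filtering the overlapping actor.
; The construction script sets the sphere radius from SetActivationRadius.
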(event OnComponentBeginOverlap(ActivateHit)
  (params (OverlappedComponent :type Primitive%20Component%20Object%20Reference) (OtherActor :type Actor%20Object%20Reference) (OtherComp :type Primitive%20Component%20Object%20Reference) (OtherBodyIndex :type Integer) (bFromSweep :type Boolean) (SweepResult :type Hit%20Result%20Structure%20%28by%20ref%29))
  (bind _textrender (Variables|Default|GetTextRender))
  ;[1 1 1] Makes sure the activation only runs ones per Hit
  (Utilities|FlowControl|Sequence
    (:then_0
      (Utilities|FlowControl|DoOnce false
        (:Completed
          ;[1 1 1] Sets May Teleport active in the Teleporter BP
          (bind _outactors (Actor|GetAllActorsOfClass "/Game/Teleports/Blueprints/Teleporter.Teleporter_C"))
          (bind _array_element (Utilities|Array|ForEachLoopwithBreak _outactors)
            (:LoopBody
              (Variables|/Game/Teleports/Blueprints/Teleporter.Teleporter_C|SetMayTeleport _array_element true)
              ;[1 1 1] Show and Hides explenation Text for Input Event
              (Rendering|SetVisibility _textrender true false))))))
    (:then_1
      (Utilities|FlowControl|DoOnce false) ; enters at Reset
    )))

(event OnComponentEndOverlap(ActivateHit)
  (params (OverlappedComponent :type Primitive%20Component%20Object%20Reference) (OtherActor :type Actor%20Object%20Reference) (OtherComp :type Primitive%20Component%20Object%20Reference) (OtherBodyIndex :type Integer))
  (bind _textrender (Variables|Default|GetTextRender))
  ;[1 1 1] Makes sure the activation only runs ones per Hit
  (Utilities|FlowControl|Sequence
    (:then_0
      (Utilities|FlowControl|DoOnce false) ; enters at Reset
    )
    (:then_1
      (Utilities|FlowControl|DoOnce false
        (:Completed
          ;[1 1 1] Sets May Teleport active in the Teleporter BP
          (bind _outactors (Actor|GetAllActorsOfClass "/Game/Teleports/Blueprints/Teleporter.Teleporter_C"))
          (bind _array_element (Utilities|Array|ForEachLoopwithBreak _outactors)
            (:LoopBody
              (Variables|/Game/Teleports/Blueprints/Teleporter.Teleporter_C|SetMayTeleport _array_element false)
              ;[1 1 1] Show and Hides explenation Text for Input Event
              (Rendering|SetVisibility _textrender false false))))))))

(fn ConstructionScript
  ;[1 1 1] Menualy adjust activation radius
  (Components|Sphere|SetSphereRadius (Variables|Default|GetActivateHit) (Variables|Activator|GetSetActivationRadius) true))